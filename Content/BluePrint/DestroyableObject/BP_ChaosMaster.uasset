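; BP_ChaosMaster is a Chaos destructible object, apparently a base class, that awards score when broken.
; The first removal event from its Geometry Collection adds Point to GameStateScore through a DoOnce gate, then starts a timer that destroys the actor after ObjectDisappearTime.
; Getter functions expose the score value and object type, though GetObjectType0 returns a fixed enum entry instead of the variable.
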(event `self.ReceiveBeginPlay`)

(event `self.GeometryCollectionComponent.OnChaosRemovalEvent`
  (params (RemovalEvent :type "ChaosRemovalEvent Structure (by ref)"))
  ;[1 1 1] 破壊された時のイベント
  (`/Engine/EditorBlueprintResources/StandardMacros.DoOnce` false
    (:`Completed`
      (bind _asgame_state_score (cast `/Game/GameState/GameStateScore` (`GameplayStatics.GetGameState`)))
      (`/Game/GameState/GameStateScore.AddScore` _asgame_state_score (`self.Point`))
      (`KismetSystemLibrary.K2_SetTimer` null "ObjectDisappear" (`self.ObjectDisappearTime`)))))

(event `ObjectDisappear`
  ;[1 1 1] 破壊された時のイベント
  (`self.K2_DestroyActor`))

(fn `GetObjectType`
  (returns (ObjectType :type "/Game/Enum/E_ObjectType Enum"))
  (return (`self.ObjectType`)))

(fn `GetObjectType_0`
  (returns (ObjectType :type "/Game/Enum/E_ObjectType Enum"))
  (return "NewEnumerator0"))

(fn `GetScore`
  (returns (Point :type Integer))
  (return (`self.Point`)))

(fn `UserConstructionScript`)